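; Security camera actor that moves and raises an audible alarm when overlapped.
; Tick plays the CamFlight timeline, whose track value is added to the root's relative X location on each update.
; Any overlap, provided player 0 is a ThirdPersonCharacter, plays the alarm cue and reports a long-range AI noise event at the camera.
; The IsAlarming flag then blocks retriggering until a cooldown delay ends.
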(event `self.ReceiveTick`
  (params (DeltaSeconds :type "Float (single-precision)"))
  (bind (_direction _newtrack_1) (`Timeline|CamFlight`)
    (:`Update`
      (`SceneComponent.K2_AddRelativeLocation` (`self.DefaultSceneRoot`) (`KismetMathLibrary.MakeVector` _newtrack_1) false false)
      (`KismetSystemLibrary.Delay` 6.0))))

(event `self.ReceiveBeginPlay`)

(event `self.ReceiveActorBeginOverlap`
  (params (OtherActor :type "Actor Object Reference"))
  (bind _returnvalue (`SceneComponent.K2_GetComponentLocation` (`self.DefaultSceneRoot`)))
  (if (not (`self.is_Alarming`))
    (cast `/Game/ThirdPersonBP/Blueprints/ThirdPersonCharacter` (`GameplayStatics.GetPlayerCharacter` 0))
    (`GameplayStatics.PlaySoundAtLocation` "/Game/Audio/Alarm_Cue.Alarm_Cue" _returnvalue (struct) 1.0 1.0 0.0 null null null)
    (`AISense_Hearing.ReportNoiseEvent` _returnvalue 1.0 null 10000.0)
    (set `self.is_Alarming` true)
    (`KismetSystemLibrary.Delay` 20.0)
    (set `self.is_Alarming` false)))

(fn `UserConstructionScript`)