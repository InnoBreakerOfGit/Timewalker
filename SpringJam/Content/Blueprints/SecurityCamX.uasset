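; SecurityCamX is a moving security camera actor that raises an alarm when overlapped.
; Each Tick plays the CamFlight timeline, whose track is added to the root's local Y position on every update.
; An overlap plays an alarm sound and reports a long-range AI noise event, then locks out retriggering for a delay.
; The cast checks player 0's character rather than the overlapping actor.
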(event `self.ReceiveTick`
  (params (DeltaSeconds :type "Float (single-precision)"))
  (bind (_direction _newtrack_1) (`Timeline|CamFlight`)
    (:`Update`
      (`SceneComponent.K2_AddRelativeLocation` (`self.DefaultSceneRoot`) (`KismetMathLibrary.MakeVector` 0.0 _newtrack_1) false false)
      (`KismetSystemLibrary.Delay` 6.0))))

(event `self.ReceiveBeginPlay`)

(event `self.ReceiveActorBeginOverlap`
  (params (OtherActor :type "Actor Object Reference"))
  (if (not (`self.is_Alarming`))
    (cast `/Game/ThirdPersonBP/Blueprints/ThirdPersonCharacter` (`GameplayStatics.GetPlayerCharacter` 0))
    (`GameplayStatics.PlaySoundAtLocation` "/Game/Audio/Alarm_Cue.Alarm_Cue" (`SceneComponent.K2_GetComponentLocation` (`self.DefaultSceneRoot`)) (struct) 1.0 1.0 0.0 null null null)
    (`AISense_Hearing.ReportNoiseEvent` (0.0 0.0 0.0) 1.0 null 10000.0)
    (set `self.is_Alarming` true)
    (`KismetSystemLibrary.Delay` 20.0)
    (set `self.is_Alarming` false)))

(fn `UserConstructionScript`)