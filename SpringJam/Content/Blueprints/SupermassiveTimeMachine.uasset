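; Time machine actor that serves as a destructible objective, setting the player's victory flag when destroyed.
; On overlap with a LazerProjectile, it checks that the player character's IsTimeMachineDestructible flag is set, then fires once.
; Destruction plays explosion effects and lingering smoke on Machine01, removes the two bottom sphere components, sets IsVictorious on the ThirdPersonCharacter, and plays the MissionFailed sound.
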(event `self.ReceiveActorBeginOverlap`
  (params (OtherActor :type "Actor Object Reference"))
  (bind _machine01 (`self.machine01`))
  ;[1 1 1] Destruction
  (bind _asthird_person_character (cast `/Game/ThirdPersonBP/Blueprints/ThirdPersonCharacter` (`GameplayStatics.GetPlayerCharacter` 0)))
  (if (`/Game/ThirdPersonBP/Blueprints/ThirdPersonCharacter.is_TimeMachineDestructible` _asthird_person_character)
    (cast `/Game/Characters/Enemy/LazerProjectile` OtherActor)
    (`/Engine/EditorBlueprintResources/StandardMacros.DoOnce` false
      (:`Completed`
        ;;[1 1 1] Explosion
        (`GameplayStatics.PlaySoundAtLocation` "/Game/StarterContent/Audio/Explosion_Cue.Explosion_Cue" (`SceneComponent.K2_GetComponentLocation` (`self.machine01`)) (struct) 1.0 1.0 0.0 null null null)
        (`GameplayStatics.SpawnEmitterAttached` "/Game/StarterContent/Particles/P_Explosion.P_Explosion" _machine01 "None" (0.0 0.0 0.0) (struct) (10.0 10.0 10.0))
        (`GameplayStatics.SpawnEmitterAttached` "/Game/StarterContent/Particles/P_Smoke.P_Smoke" _machine01 "None" (0.0 0.0 0.0) (struct) (8.0 8.0 8.0) "KeepRelativeOffset" false)
        (`ActorComponent.K2_DestroyComponent` (`self.sphere_bottom1`))
        (`ActorComponent.K2_DestroyComponent` (`self.sphere_bottom`))
        (bind _asthird_person_character_2 (cast `/Game/ThirdPersonBP/Blueprints/ThirdPersonCharacter` (`GameplayStatics.GetPlayerCharacter` 0)))
        (set `/Game/ThirdPersonBP/Blueprints/ThirdPersonCharacter.is_victorious` true _asthird_person_character_2)
        (`GameplayStatics.PlaySoundAtLocation` "/Game/Audio/MissionFailed.MissionFailed" (0.0 0.0 0.0) (struct) 1.0 1.0 0.0 null null null)))))

(fn `UserConstructionScript`)