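; Destructible machine actor that plays a gearwheel sound at start and blows up when a LazerProjectile overlaps it.
; The one-time hit plays explosion sound, fire and smoke effects, removes the SphereBottom and Outer components, and calls DestroyMachine on the player's ThirdPersonCharacter.
; Tick shows WidgetButton while the player's IsLookingAtItem flag is set and they are within ItemRange, rotating it toward the character's location.
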(event `self.ReceiveBeginPlay`
  ;[1 1 1] Destruction
  (`GameplayStatics.PlaySoundAtLocation` "/Game/Audio/Gearwheel_Cue.Gearwheel_Cue" (`SceneComponent.K2_GetComponentLocation` (`self.machine_destroyable01`)) (struct) 1.0 1.0 0.0 null null null))

(event `self.ReceiveActorBeginOverlap`
  (params (OtherActor :type "Actor Object Reference"))
  (bind _machine_destroyable01 (`self.machine_destroyable01`))
  ;[1 1 1] Destruction
  (cast `/Game/Characters/Enemy/LazerProjectile` OtherActor)
  (`/Engine/EditorBlueprintResources/StandardMacros.DoOnce` false
    (:`Completed`
      ;;[1 1 1] Explosion
      (`GameplayStatics.PlaySoundAtLocation` "/Game/StarterContent/Audio/Explosion_Cue.Explosion_Cue" (`SceneComponent.K2_GetComponentLocation` (`self.machine_destroyable01`)) (struct) 1.0 1.0 0.0 null null null)
      (`GameplayStatics.SpawnEmitterAttached` "/Game/StarterContent/Particles/P_Explosion.P_Explosion" _machine_destroyable01 "None" (0.0 0.0 0.0) (struct) (10.0 10.0 10.0))
      (`GameplayStatics.SpawnEmitterAttached` "/Game/StarterContent/Particles/P_Smoke.P_Smoke" _machine_destroyable01 "None" (0.0 0.0 0.0) (struct) (8.0 8.0 8.0) "KeepRelativeOffset" false)
      (`ActorComponent.K2_DestroyComponent` (`self.sphere_bottom`))
      (`ActorComponent.K2_DestroyComponent` (`self.Outer`))
      (if (not (`self.is_MachineDestroyed`))
        (bind _asthird_person_character (cast `/Game/ThirdPersonBP/Blueprints/ThirdPersonCharacter` (`GameplayStatics.GetPlayerCharacter` 0)))
        (`/Game/ThirdPersonBP/Blueprints/ThirdPersonCharacter.DestroyMachine` _asthird_person_character)
        (set `self.is_MachineDestroyed` true)))))

(event `self.ReceiveTick`
  (params (DeltaSeconds :type "Float (single-precision)"))
  (bind _widget_button (`self.Widget_Button`))
  ;[1 1 1] Wenn man sich in der Nähe aufhält wird das Widget sichtbar
  (bind _asthird_person_character (cast `/Game/ThirdPersonBP/Blueprints/ThirdPersonCharacter` (`GameplayStatics.GetPlayerCharacter` 0)))
  (if (`/Game/ThirdPersonBP/Blueprints/ThirdPersonCharacter.is_LookingAtItem` _asthird_person_character)
    (if (< (`KismetMathLibrary.VSize` (- (`self.K2_GetActorLocation` (`GameplayStatics.GetPlayerCharacter` 0)) (`self.K2_GetActorLocation`))) (`/Game/ThirdPersonBP/Blueprints/ThirdPersonCharacter.item_range` _asthird_person_character))
      (`SceneComponent.SetVisibility` _widget_button true false)
      ;[1 1 1] Richtet das Widget nach der Player Camera aus
      (`SceneComponent.K2_SetWorldRotation` (`self.Widget_Button`) (`KismetMathLibrary.FindLookAtRotation` (`self.K2_GetActorLocation`) (`self.K2_GetActorLocation` (`GameplayStatics.GetPlayerCharacter` 0))) false false)
      (else
        (`SceneComponent.SetVisibility` _widget_button false false :!label _label)))
    (else
      (goto _label))))

(fn `UserConstructionScript`)